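; DeliverySystem is a conveyor actor that carries Package actors along the direction of its Arrow component.
; Box overlap events add and remove packages from the ConveyorPackages array.
; Each Tick offsets every package not being held along the Arrow's forward vector by ConveyorSpeed scaled by delta time, without sweeping.
; GetSpawnPos exposes the Arrow's world location as a spawn position.
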(event `self.Box.OnComponentBeginOverlap`
  (params (OverlappedComponent :type "PrimitiveComponent Object Reference") (OtherActor :type "Actor Object Reference") (OtherComp :type "PrimitiveComponent Object Reference") (OtherBodyIndex :type Integer) (bFromSweep :type Boolean) (SweepResult :type "HitResult Structure (by ref)"))
  (bind _aspackage (cast `/Game/Blueprints/Package` OtherActor))
  (`KismetArrayLibrary.Array_Add` (`self.ConveyorPackages`) _aspackage)
  (`KismetSystemLibrary.PrintString` "Package on Conveyor"))

(event `self.Box.OnComponentEndOverlap`
  (params (OverlappedComponent :type "PrimitiveComponent Object Reference") (OtherActor :type "Actor Object Reference") (OtherComp :type "PrimitiveComponent Object Reference") (OtherBodyIndex :type Integer))
  (bind _aspackage (cast `/Game/Blueprints/Package` OtherActor))
  (`KismetArrayLibrary.Array_RemoveItem` (`self.ConveyorPackages`) _aspackage))

(event `self.ReceiveTick`
  (params (DeltaSeconds :type "Float (single-precision)"))
  (for _array_element (`self.ConveyorPackages`)
    (if (not (`/Game/Blueprints/Package.BeingHeld` _array_element))
      (`self.K2_AddActorWorldOffset` _array_element (* (`SceneComponent.GetForwardVector` (`self.Arrow`)) (* (`self.ConveyorSpeed`) (`GameplayStatics.GetWorldDeltaSeconds`))) false false))))

(fn `GetSpawnPos`
  (returns (SpawnPos :type "Vector Structure"))
  (return (`SceneComponent.K2_GetComponentLocation` (`self.Arrow`))))

(fn `UserConstructionScript`)