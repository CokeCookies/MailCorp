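; Game mode for a package sorting game that spawns packages and scores their delivery to targets.
; On BeginPlay it caches the target and delivery systems, then a delayed DoN loop spawns the starting packages at random delivery systems.
; ScorePackage compares package and target textures, incrementing score and HUD on a match, resetting only the HUD otherwise.
; Helpers pick a random logo and append scores to a capped, unsorted high-score list.
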(event `self.ReceiveBeginPlay`
  (`|ExecutionSequence`
    (:`then_0`
      (bind _returnvalue (`GameplayStatics.GetActorOfClass` "/Game/Blueprints/SortingTarget_OLD.SortingTarget_OLD_C"))
      (set `self.SortingTarget` _returnvalue))
    (:`then_1`
      (bind _outactors (`GameplayStatics.GetAllActorsOfClass` "/Game/Blueprints/DeliverySystem.DeliverySystem_C"))
      (set `self.DeliverySystems` _outactors))
    (:`then_2`
      (`/Engine/EditorBlueprintResources/StandardMacros.Do N` (`self.StartingPackages`) :!label _label
        (:`Exit`
          (`self.SpawnNewPackage`)
          (`KismetSystemLibrary.Delay` 2.0)
          (goto _label))))))

(event `SpawnNewPackage`
  (`|SpawnActorFromClass` "/Game/Blueprints/Package.Package_C" (`KismetMathLibrary.MakeTransform` (`/Game/Blueprints/DeliverySystem.GetSpawnPos` (`KismetArrayLibrary.Array_Random` (`self.DeliverySystems`))) (struct) (0.5 0.5 0.5)) "Undefined" "OverrideRootScale" null null))

(event `ScorePackage`
  (params (Package :type "/Game/Blueprints/Package Object Reference") (Target :type "/Game/Blueprints/SortingTarget Object Reference"))
  (bind _hud_widget (`self.HUD_Widget`))
  (if (== (`/Game/Blueprints/Package.SetTexture` Package) (`/Game/Blueprints/SortingTarget.SetTexture` Target))
    (`/Engine/EditorBlueprintResources/StandardMacros.IncrementInt` (`self.Score`)
      (:`  `
        (`/Game/UI/MainHUD_Widget.IncreaseScore` _hud_widget)))
    (else
      (`/Game/UI/MainHUD_Widget.ResetScore` _hud_widget))))

(fn `GetRandomLogo`
  (returns (RandomLogo :type "Texture Object Reference") (Index :type Integer))
  (bind (_outitem _outindex) (`KismetArrayLibrary.Array_Random` (`self.Logos`)))
  (return _outitem _outindex))

(fn `UpdateHighScore`
  (`KismetArrayLibrary.Array_Add` (`self.HighScores`) (`self.Score`))
  (while (> (`KismetArrayLibrary.Array_Length` (`self.HighScores`)) 10)
    (`KismetArrayLibrary.Array_Remove` (`self.HighScores`) 10)))

(fn `UserConstructionScript`)