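; Package is a carryable box actor for a sorting game, branded with a random logo from the sorting game mode.
; The construction script applies that logo through a dynamic material instance, and BeginPlay puts the cube on a custom collision channel.
; While held, it teleports each tick to the first-person player's package position.
; When loose and fallen below a kill height, it asks the game mode for a replacement and destroys itself.
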(event `self.ReceiveBeginPlay`
  (`PrimitiveComponent.SetCollisionObjectType` (`self.Cube`) "ECC_GameTraceChannel2"))

(event `self.ReceiveTick`
  (params (DeltaSeconds :type "Float (single-precision)"))
  (bind (_returnvalue_x _returnvalue_y _returnvalue_z) (`KismetMathLibrary.BreakVector` (`self.K2_GetActorLocation`)))
  (if (`self.BeingHeld`)
    (bind _player (`/Game/Blueprints/FunctionLibrary.GetFPPlayer`))
    (`self.K2_SetActorLocation` (`/Game/FirstPersonBP/Blueprints/FirstPersonCharacter.GetPackagePos` _player self) false true)
    (elif (< _returnvalue_z -1000.0)
      (bind _sortinggamemode (`/Game/Blueprints/FunctionLibrary.GetSortingGameMode`))
      (`/Game/Blueprints/Sorting_GameMode.SpawnNewPackage` _sortinggamemode)
      (`self.K2_DestroyActor`))))

(fn `UserConstructionScript`
  (bind _sortinggamemode (`/Game/Blueprints/FunctionLibrary.GetSortingGameMode`))
  (bind _returnvalue (`PrimitiveComponent.CreateDynamicMaterialInstance` (`self.Cube`) 0 "/Game/Materials/Cube_Material.Cube_Material" "None"))
  (bind _randomlogo (`/Game/Blueprints/Sorting_GameMode.GetRandomLogo` _sortinggamemode))
  (set `self.SetTexture` _randomlogo)
  (`MaterialInstanceDynamic.SetTextureParameterValue` _returnvalue "LogoTexture" _randomlogo))