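; SortingTarget is a drop target in a package-sorting game, showing a random logo from the sorting game mode on its Plane.
; BeginPlay creates a dynamic material for the logo texture and records it in SetTexture.
; A Package overlapping the Box is scored by the game mode, and the Plane toggles visibility around TargetDelay.
; The logo then rerolls, with material and SetTexture fed by separate GetRandomLogo calls.
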(event `self.ReceiveBeginPlay`
  (bind _returnvalue (`PrimitiveComponent.CreateDynamicMaterialInstance` (`self.Plane`) 0 "/Game/Materials/Cube_Material.Cube_Material" "None"))
  (bind _sortinggamemode (`/Game/Blueprints/FunctionLibrary.GetSortingGameMode`))
  (bind _output_get (set `self.SetTexture` (`/Game/Blueprints/Sorting_GameMode.GetRandomLogo` _sortinggamemode)))
  (`MaterialInstanceDynamic.SetTextureParameterValue` _returnvalue "LogoTexture" _output_get)
  (set `self.MaterialInstance` _returnvalue))

(event `self.Box.OnComponentBeginOverlap`
  (params (OverlappedComponent :type "PrimitiveComponent Object Reference") (OtherActor :type "Actor Object Reference") (OtherComp :type "PrimitiveComponent Object Reference") (OtherBodyIndex :type Integer) (bFromSweep :type Boolean) (SweepResult :type "HitResult Structure (by ref)"))
  (bind _aspackage (cast `/Game/Blueprints/Package` OtherActor))
  (bind _sortinggamemode (`/Game/Blueprints/FunctionLibrary.GetSortingGameMode`))
  (`/Game/Blueprints/Sorting_GameMode.ScorePackage` _sortinggamemode _aspackage self)
  (`SceneComponent.ToggleVisibility` (`self.Plane`) false)
  (`KismetSystemLibrary.Delay` (`self.TargetDelay`))
  (`SceneComponent.ToggleVisibility` (`self.Plane`) false)
  (bind _randomlogo (`/Game/Blueprints/Sorting_GameMode.GetRandomLogo` _sortinggamemode))
  (`MaterialInstanceDynamic.SetTextureParameterValue` (`self.MaterialInstance`) "LogoTexture" _randomlogo)
  (set `self.SetTexture` _randomlogo))

(fn `UserConstructionScript`)